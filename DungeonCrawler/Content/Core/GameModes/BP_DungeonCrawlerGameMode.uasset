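; Dungeon crawler game mode that switches the player camera between following the character and framing the room the player is in.
; Entering a room detaches the camera and instantly moves it above the grid manager's computed room center, raised by the spring arm's length.
; Exiting a room reattaches the camera to the player's spring arm, snapping its location while keeping world rotation.
; Other level events only forward to the parent implementation.
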(event EventBeginPlay
  (Variables|Default|SetGrid%20Manager (Class|DungeonCrawlerGameState|GetGridManager (Variables|Default|GetDungeonGameState))))

(event EventOnGridManagerInitialized
  (|CallParentFunction)
  (Variables|Default|SetPlayer%20Camera%20Component (Actor|GetComponentbyClass (Variables|Default|GetPlayerCharacterZD) "/Script/Engine.CameraComponent")))

(event EventOnEndOfLevelReached
  (|CallParentFunction))

(event EventOnLevelSequenceGenerated
  (|CallParentFunction))

(event EventOnLevelIndexChanged
  (|CallParentFunction))

(event EventOnPlayerEnteredRoom
  (|CallParentFunction)
  (Camera|Camera:RoomMode))

(event EventOnPlayerExitedRoom
  (|CallParentFunction)
  (Camera|Camera:FollowMode))

(fn ConstructionScript)

(fn Camera:RoomMode
  (bind _playercharacterzd (Variables|Default|GetPlayerCharacterZD))
  (bind _grid_manager (Variables|Default|GetGrid%20Manager))
  (bind _currentposition (Variables|/Script/DungeonCrawler.BaseCharacterZD|GetCurrentPosition _playercharacterzd))
  (bind _outroomtiles (Class|GridManager|GetRoomTiles _grid_manager _currentposition))
  (bind _returnvalue (Class|GridManager|FindRoomCenter _grid_manager _outroomtiles))
  (bind _returnvalue_2 (Class|GridManager|GridtoWorldPosition _grid_manager _returnvalue true))
  ;[1 1 1] Instant switch
  (LocalVariables|SetSpring%20Arm%20Length (Variables|/Script/Engine.SpringArmComponent|GetTargetArmLength (Actor|GetComponentbyClass (Variables|Default|GetPlayerCharacterZD) "/Script/Engine.SpringArmComponent")))
  (bind _output_get (LocalVariables|SetPlayerCameraComponent (Actor|GetComponentbyClass (Variables|Default|GetPlayerCharacterZD) "/Script/Engine.CameraComponent")))
  (Transformation|DetachFromComponent _output_get "KeepWorld" "KeepWorld" "KeepWorld" true)
  (Transformation|SetWorldLocation _output_get (Math|Vector|MakeVector (.x _returnvalue_2) (.y _returnvalue_2) (+ (.z _returnvalue_2) (LocalVariables|GetSpring%20Arm%20Length))) false false)
  (return))

(fn Camera:FollowMode
  (Transformation|AttachComponentToComponent (Variables|Default|GetPlayer%20Camera%20Component) (Actor|GetComponentbyClass (Variables|Default|GetPlayerCharacterZD) "/Script/Engine.SpringArmComponent") "None" "SnapToTarget" "KeepWorld" "KeepWorld" true)
  (return))