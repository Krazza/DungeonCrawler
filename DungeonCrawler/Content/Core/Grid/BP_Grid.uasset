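; BP_Grid is a tile grid actor whose construction script prepares line and selection visuals from row, column and tile-size settings.
; Two dynamic instances of M_Grid receive separate color and opacity values for lines and selection.
; Loops compute each row and column line's endpoints and pass them to CreateLine, which is still empty.
; Tile conversion, selection and validity functions are also stubs, and no events run logic.
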(event EventBeginPlay)

(event Collision|EventActorBeginOverlap
  (params (OtherActor :type Actor%20Object%20Reference)))

(event EventTick
  (params (DeltaSeconds :type Float%20%28single-precision%29)))

(fn ConstructionScript
  (bind _material_instance (Private|CreateMaterialInstance (Variables|Constants|GetLine%20Color) (Variables|Constants|GetLine%20Opacity)))
  (LocalVariables|SetLines%20Material%20Instance _material_instance)
  (bind _material_instance_2 (Private|CreateMaterialInstance (Variables|Constants|GetSelection%20Color) (Variables|Constants|GetSelection%20Opacity)))
  (LocalVariables|SetSelection%20Material%20Instance _material_instance_2)
  (Utilities|FlowControl|Sequence
    (:then_0
      ;[1 1 1] create horizontal lines geometry
      (for _index (range 0 (Variables|Constants|GetNum%20Rows))
        (LocalVariables|SetLine%20Start (* _index (Variables|Constants|GetTile%20Size)))
        (LocalVariables|SetLine%20End (Private|GetGridWidth))
        (Private|CreateLine (Math|Vector|MakeVector (LocalVariables|GetLine%20Start) 0.0 0.0) (Math|Vector|MakeVector (LocalVariables|GetLine%20Start) (LocalVariables|GetLine%20End) 0.0) (Variables|Constants|GetLine%20Thickness) (LocalVariables|GetLine%20Vertices) (LocalVariables|GetLine%20Triangles))))
    (:then_1
      ;[1 1 1] create horizontal lines geometry
      (for _index_2 (range 0 (Variables|Constants|GetNum%20Columns))
        (LocalVariables|SetLine%20Start (* _index_2 (Variables|Constants|GetTile%20Size)))
        (LocalVariables|SetLine%20End (Private|GetGridHeight))
        (Private|CreateLine (Math|Vector|MakeVector 0.0 (LocalVariables|GetLine%20Start) 0.0) (Math|Vector|MakeVector (LocalVariables|GetLine%20End) (LocalVariables|GetLine%20Start) 0.0) (Variables|Constants|GetLine%20Thickness) (LocalVariables|GetLine%20Vertices) (LocalVariables|GetLine%20Triangles))))))

(fn CreateLine
  (params (Start%20Position :type Vector) (End%20Position :type Vector) (Line%20Thickness :type Float%20%28double-precision%29) (Vertices :type Array%20of%20Vectors) (Triangles :type Array%20of%20Integers)))

(fn GetGridWidth
  (return (* (Variables|Constants|GetNum%20Columns) (Variables|Constants|GetTile%20Size))))

(fn GetGridHeight
  (return (* (Variables|Constants|GetNum%20Rows) (Variables|Constants|GetTile%20Size))))

(fn CreateMaterialInstance
  (params (Color :type Linear%20Color%20Structure) (Opacity :type Float%20%28double-precision%29))
  (bind _returnvalue (Rendering|Material|CreateDynamicMaterialInstance "/Game/Core/Grid/Materials/M_Grid.M_Grid" "None" "None" :!class /Script/Engine.KismetMaterialLibrary))
  (Rendering|Material|SetVectorParameterValue _returnvalue "Color" Color :!class /Script/Engine.MaterialInstanceDynamic)
  (Rendering|Material|SetScalarParameterValue _returnvalue "Opacity" Opacity :!class /Script/Engine.MaterialInstanceDynamic)
  (return _returnvalue))

(fn LocationtoTilePosition
  (params (Location :type Vector))
  (return "" false))

(fn TilePositiontoLocation
  (params (Tile%20Position :type Int%20Point%20Structure) (isCenter :type Boolean))
  (return false ""))

(fn SetSelectedTile
  (params (Tile%20Position :type Int%20Point%20Structure)))